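; VR game mode for a one- or two-player Oculus match, running login, calibration, rounds and scoring.
; Login assigns controllers to tagged bodies, and calibration opens a DoOnce that starts the round, with an optional timed demo fade-out.
; Pawn defeats update BP_Scoreboard and lead to a respawn or, at the winning score, a match reset.
; SpawnAndPossessPlayer's spawn-and-possess nodes are disconnected from its entry.
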(event Custom|ForceStart
  (bind _scoreboard (Variables|Default|GetScoreboard))
  (bind _player_1 (Variables|Default|GetPlayer%201))
  (bind _player_2 (Variables|Default|GetPlayer%202))
  ;[1 1 1] Round and Match Flow
  (Development|PrintString "Forcing Start")
  (Variables|/Game/Blueprints/ScoreBoard/BP_Scoreboard.BP_Scoreboard_C|SetPlayer%201%20Calibrated _scoreboard true)
  (Variables|/Game/Blueprints/ScoreBoard/BP_Scoreboard.BP_Scoreboard_C|SetPlayer%202%20Calibrated _scoreboard true)
  (Utilities|FlowControl|Sequence
    (:then_0
      (goto _label Reset))
    (:then_1
      (Utilities|FlowControl|DoOnce false :!label _label
        (:Completed
          (Variables|Default|SetbRoundStarted true)
          (Game|Player|SetViewTargetwithBlend _player_1 (Variables|/Game/Blueprints/Game/Oculus_PlayerController.Oculus_PlayerController_C|GetMyBody _player_1) 0.0 "VTBlend_Linear" 0.0 false)
          (Utilities|IsValid _player_2
            (:Is%20Valid
              (Game|Player|SetViewTargetwithBlend _player_2 (Variables|/Game/Blueprints/Game/Oculus_PlayerController.Oculus_PlayerController_C|GetMyBody _player_2) 0.0 "VTBlend_Linear" 0.0 false))
            (:Is%20Not%20Valid
              _))
          (CallFunction|SpawnPawnsforPlayers)
          (if (Variables|Default|GetbDemoMode)
            (Utilities|Time|SetTimerbyFunctionName 0 "FadeToBlack" (Variables|Default|GetFadeToBlackTime))))))))

(event Custom|SetFadeToBlackTime
  (params (FadeTime :type Float%20%28single-precision%29))
  ;[1 1 1] Resetting Logic
  ;;[1 1 1] Fading to Black
  (Variables|Default|SetFadeToBlackTime FadeTime))

(event Custom|SpawnPawnsForPlayers
  (bind _player_2 (Variables|Default|GetPlayer%202))
  (bind _player_2_2 (Variables|Default|GetPlayer%202))
  ;[1 1 1] Player Spawning
  ;;[1 1 1] Clean up the other players
  (Utilities|IsValid _player_2_2
    (:Is%20Valid
      (Actor|DestroyActor (Pawn|GetControlledPawn _player_2_2)))
    (:Is%20Not%20Valid
      _))
  (Actor|DestroyActor (Pawn|GetControlledPawn (Variables|Default|GetPlayer%201)))
  (CallFunction|ResetProps)
  (bind _pawn (CallFunction|SpawnandPossessPlayer (Variables|Default|GetPlayer%201)))
  (EventDispatchers|BindEventtoDefeated _pawn (delegate Custom|Defeated_Event))
  (Utilities|IsValid _player_2
    (:Is%20Valid
      (bind _pawn_2 (CallFunction|SpawnandPossessPlayer _player_2))
      (EventDispatchers|BindEventtoDefeated _pawn_2 (delegate Custom|Defeated_Event))
      (Utilities|FlowControl|Delay 0.2)
      (Default|GetPawns (Variables|Default|GetPlayer%201%20Body))
      (Default|GetPawns (Variables|Default|GetPlayer%202%20Body)))))

(event Custom|Defeated_Event
  (params (Owner :type Oculus%20Player%20Controller%20Object%20Reference))
  (bind _scoreboard (Variables|Default|GetScoreboard))
  (bind _player_2 (Variables|Default|GetPlayer%202))
  (bind _player_1 (Variables|Default|GetPlayer%201))
  (bind _returnvalue (Pawn|GetControlledPawn _player_2))
  ;[1 1 1] Player Was Defeated
  (if (== Owner (Variables|Default|GetPlayer%201))
    ;;[1 1 1] Increment Player Score
    (Variables|/Game/Blueprints/ScoreBoard/BP_Scoreboard.BP_Scoreboard_C|SetPlayer%202%20Score _scoreboard (+ (Variables|/Game/Blueprints/ScoreBoard/BP_Scoreboard.BP_Scoreboard_C|GetPlayer%202%20Score _scoreboard) 1))
    (bind _asbp_player_character_pawn (Utilities|Casting|CastToBP_Player_Character_Pawn _returnvalue)
      (:then
        (Default|Victorious _asbp_player_character_pawn)
        (Input|DisableInput _returnvalue _player_2))
      (:CastFailed
        _))
    (else
      (Variables|/Game/Blueprints/ScoreBoard/BP_Scoreboard.BP_Scoreboard_C|SetPlayer%201%20Score _scoreboard (+ (Variables|/Game/Blueprints/ScoreBoard/BP_Scoreboard.BP_Scoreboard_C|GetPlayer%201%20Score _scoreboard) 1))
      (bind _asbp_player_character_pawn_2 (Utilities|Casting|CastToBP_Player_Character_Pawn (Pawn|GetControlledPawn _player_1))
        (:then
          (Default|Victorious _asbp_player_character_pawn_2)
          (Input|DisableInput _asbp_player_character_pawn_2 _player_1))
        (:CastFailed
          _))))
  (Utilities|FlowControl|RetriggerableDelay 8.0)
  (CallFunction|HidePlayers)
  (CallFunction|NextRound))

(event Custom|Next%20Round
  (bind _winning_score (Variables|Default|GetWinning%20Score))
  (bind _scoreboard (Variables|Default|GetScoreboard))
  (bind _player_1 (Variables|Default|GetPlayer%201))
  (bind _player_2 (Variables|Default|GetPlayer%202))
  (bind _scoreboard_2 (Variables|Default|GetScoreboard))
  ;[1 1 1] Round and Match Flow
  (if (or (== (Variables|/Game/Blueprints/ScoreBoard/BP_Scoreboard.BP_Scoreboard_C|GetPlayer%201%20Score _scoreboard) _winning_score) (== _winning_score (Variables|/Game/Blueprints/ScoreBoard/BP_Scoreboard.BP_Scoreboard_C|GetPlayer%202%20Score _scoreboard)))
    (Default|PlayerWins _scoreboard_2)
    (Utilities|FlowControl|Delay 8.0)
    (Default|ResetScoreboard _scoreboard_2)
    (CallFunction|Reset)
    (Utilities|FlowControl|DoOnce false) ; enters at Reset
    (else
      (CallFunction|SpawnPawnsforPlayers))))

(event Custom|PlayerReady
  (params (Player :type Oculus%20Player%20Controller%20Object%20Reference))
  (bind _scoreboard (Variables|Default|GetScoreboard))
  (bind _scoreboard_2 (Variables|Default|GetScoreboard))
  ;[1 1 1] Player Login and Calibration Flow
  ;;[1 1 1] Player Ready
  (Utilities|SwitchonPlayer Player
    (:Player%201
      (if (Variables|/Game/Blueprints/ScoreBoard/BP_Scoreboard.BP_Scoreboard_C|GetPlayer%201%20Calibrated _scoreboard)
        (Variables|/Game/Blueprints/ScoreBoard/BP_Scoreboard.BP_Scoreboard_C|SetPlayer%201%20Ready _scoreboard_2 true)))
    (:Player%202
      (if (Variables|/Game/Blueprints/ScoreBoard/BP_Scoreboard.BP_Scoreboard_C|GetPlayer%202%20Calibrated _scoreboard)
        (Variables|/Game/Blueprints/ScoreBoard/BP_Scoreboard.BP_Scoreboard_C|SetPlayer%202%20Ready _scoreboard_2 true)))))

(event Custom|PlayerCalibrated
  (params (Player :type Oculus%20Player%20Controller%20Object%20Reference))
  (bind _player_1 (Variables|Default|GetPlayer%201))
  (bind _player_2 (Variables|Default|GetPlayer%202))
  (bind _scoreboard (Variables|Default|GetScoreboard))
  (bind _scoreboard_2 (Variables|Default|GetScoreboard))
  ;[1 1 1] Round and Match Flow
  (Utilities|SwitchonPlayer Player
    (:Player%201
      (Variables|/Game/Blueprints/ScoreBoard/BP_Scoreboard.BP_Scoreboard_C|SetPlayer%201%20Calibrated _scoreboard_2 true))
    (:Player%202
      (Variables|/Game/Blueprints/ScoreBoard/BP_Scoreboard.BP_Scoreboard_C|SetPlayer%202%20Calibrated _scoreboard_2 true)))
  (Variables|/Game/Assets/VR/Oculus_Character_Actor.Oculus_Character_Actor_C|SetbHasPlayer (Variables|/Game/Blueprints/Game/Oculus_PlayerController.Oculus_PlayerController_C|GetMyBody Player) true)
  (if (or (and (Variables|/Game/Blueprints/ScoreBoard/BP_Scoreboard.BP_Scoreboard_C|GetPlayer%201%20Calibrated _scoreboard) (Variables|/Game/Blueprints/ScoreBoard/BP_Scoreboard.BP_Scoreboard_C|GetPlayer%202%20Calibrated _scoreboard)) (== (Variables|Default|GetPlayer%202) 0))
    (Utilities|FlowControl|DoOnce false
      (:Completed
        (Variables|Default|SetbRoundStarted true)
        (Game|Player|SetViewTargetwithBlend _player_1 (Variables|/Game/Blueprints/Game/Oculus_PlayerController.Oculus_PlayerController_C|GetMyBody _player_1) 0.0 "VTBlend_Linear" 0.0 false)
        (Utilities|IsValid _player_2
          (:Is%20Valid
            (Game|Player|SetViewTargetwithBlend _player_2 (Variables|/Game/Blueprints/Game/Oculus_PlayerController.Oculus_PlayerController_C|GetMyBody _player_2) 0.0 "VTBlend_Linear" 0.0 false))
          (:Is%20Not%20Valid
            _))
        (CallFunction|SpawnPawnsforPlayers)
        (if (Variables|Default|GetbDemoMode)
          (Utilities|Time|SetTimerbyFunctionName 0 "FadeToBlack" (Variables|Default|GetFadeToBlackTime)))))))

(event Custom|Reset
  (bind _scoreboard (Variables|Default|GetScoreboard))
  (bind _scoreboard_2 (Variables|Default|GetScoreboard))
  (bind _scoreboard_3 (Variables|Default|GetScoreboard))
  ;[1 1 1] Resetting Logic
  (Variables|/Game/Blueprints/ScoreBoard/BP_Scoreboard.BP_Scoreboard_C|SetPlayer%201%20Score _scoreboard_2 0)
  (Variables|/Game/Blueprints/ScoreBoard/BP_Scoreboard.BP_Scoreboard_C|SetPlayer%202%20Score _scoreboard_2 0)
  (Variables|/Game/Blueprints/ScoreBoard/BP_Scoreboard.BP_Scoreboard_C|SetPlayer%201%20Calibrated _scoreboard false)
  (Variables|/Game/Blueprints/ScoreBoard/BP_Scoreboard.BP_Scoreboard_C|SetPlayer%202%20Calibrated _scoreboard false)
  (Variables|/Game/Blueprints/ScoreBoard/BP_Scoreboard.BP_Scoreboard_C|SetPlayer%201%20Ready _scoreboard_3 false)
  (Variables|/Game/Blueprints/ScoreBoard/BP_Scoreboard.BP_Scoreboard_C|SetPlayer%202%20Ready _scoreboard_3 false)
  (Variables|/Game/Assets/VR/Oculus_Character_Actor.Oculus_Character_Actor_C|SetbHasPlayer (Variables|Default|GetPlayer%201%20Body) false)
  (Variables|/Game/Assets/VR/Oculus_Character_Actor.Oculus_Character_Actor_C|SetbHasPlayer (Variables|Default|GetPlayer%202%20Body) false)
  (CallFunction|ResetProps)
  (Utilities|Time|ClearTimerbyFunctionName 0 "FadeToBlack")
  (Variables|Default|SetbRoundStarted false))

(event Custom|HidePlayers
  ;[1 1 1] Resetting Logic
  ;;[1 1 1] Clean up the other players
  (bind _asbp_player_character_pawn (Utilities|Casting|CastToBP_Player_Character_Pawn (Pawn|GetControlledPawn (Variables|Default|GetPlayer%202)))
    (:then
      (Default|HidePawn _asbp_player_character_pawn))
    (:CastFailed
      _))
  (bind _asbp_player_character_pawn_2 (Utilities|Casting|CastToBP_Player_Character_Pawn (Pawn|GetControlledPawn (Variables|Default|GetPlayer%201))))
  (Default|HidePawn _asbp_player_character_pawn_2))

(event Custom|ResetProps
  (bind _player_2 (Variables|Default|GetPlayer%202))
  ;[1 1 1] Resetting Logic
  (Default|ResetProps (Variables|Default|GetPlayer%201))
  (Utilities|IsValid _player_2
    (:Is%20Valid
      (Default|ResetProps _player_2))))

(event Custom|TotalReset
  (bind _player_1_body (Variables|Default|GetPlayer%201%20Body))
  (bind _player_2_body (Variables|Default|GetPlayer%202%20Body))
  (bind _player_1 (Variables|Default|GetPlayer%201))
  (bind _player_2 (Variables|Default|GetPlayer%202))
  (bind _player_1_2 (Variables|Default|GetPlayer%201))
  (bind _player_2_2 (Variables|Default|GetPlayer%202))
  (bind _returnvalue (Pawn|GetControlledPawn _player_2_2))
  (bind _returnvalue_2 (Pawn|GetControlledPawn _player_1_2))
  ;[1 1 1] Resetting Logic
  (CallFunction|FadeUp)
  (CallFunction|Reset)
  (Default|ResetScoreboard (Variables|Default|GetScoreboard))
  (Utilities|FlowControl|Sequence
    (:then_0
      (Utilities|IsValid _returnvalue_2
        (:Is%20Valid
          (Actor|DestroyActor _returnvalue_2))))
    (:then_1
      (Utilities|IsValid _returnvalue
        (:Is%20Valid
          (Actor|DestroyActor _returnvalue))))
    (:then_2
      ;;[1 1 1] Reset the state of the bodies, if people disconnected
      (Utilities|IsValid (Variables|/Game/Assets/VR/Oculus_Character_Actor.Oculus_Character_Actor_C|GetPlayerController _player_1_body)
        (:Is%20Not%20Valid
          (Variables|/Game/Assets/VR/Oculus_Character_Actor.Oculus_Character_Actor_C|SetIsTaken _player_1_body false)
          (Utilities|IsValid (Variables|/Game/Assets/VR/Oculus_Character_Actor.Oculus_Character_Actor_C|GetPlayerController _player_2_body)
            (:Is%20Not%20Valid
              (Variables|/Game/Assets/VR/Oculus_Character_Actor.Oculus_Character_Actor_C|SetIsTaken _player_2_body false))))))
    (:then_3
      ;[1 1 1] Round and Match Flow
      (Utilities|FlowControl|DoOnce false) ; enters at Reset
    )))

(event Custom|FadeToBlack
  ;[1 1 1] Resetting Logic
  ;;[1 1 1] Fading to Black
  (Default|FadeOut (Variables|Default|GetPlayer%201))
  (Default|FadeOut (Variables|Default|GetPlayer%202)))

(event Custom|FadeUp
  ;[1 1 1] Resetting Logic
  ;;[1 1 1] Fading to Black
  (Default|FadeUp (Variables|Default|GetPlayer%201))
  (Default|FadeUp (Variables|Default|GetPlayer%202)))

(event EventPostLogin
  (params (NewPlayer :type Player%20Controller%20Object%20Reference))
  ;[1 1 1] Player Login and Calibration Flow
  ;;[1 1 1] Player Logged In
  (Utilities|FlowControl|Delay 0.0)
  (bind _asoculus_player_controller (Utilities|Casting|CastToOculus_PlayerController NewPlayer))
  (Utilities|IsValid (Variables|Default|GetPlayer%201) ; Is player 1 already taken?
    (:Is%20Valid
      (Utilities|IsValid (Variables|Default|GetPlayer%202) ; Is player 1 already taken?
        (:Is%20Not%20Valid
          (Variables|Default|SetPlayer%202 _asoculus_player_controller))))
    (:Is%20Not%20Valid
      (Variables|Default|SetPlayer%201 _asoculus_player_controller)))
  (bind _body (CallFunction|SelectBody _asoculus_player_controller))
  (Default|TakeBodyonServer _asoculus_player_controller _body)
  (if (and (== NewPlayer (Variables|Default|GetPlayer%202)) (Variables|Default|GetbRoundStarted))
    (CallFunction|HidePlayers)
    (CallFunction|TotalReset)))

(event EventBeginPlay
  ;[1 1 1] Player Login and Calibration Flow
  ;;[1 1 1] Grab the player starts
  (bind _outactors (Actor|GetAllActorsOfClass "/Script/Engine.PlayerStart"))
  (for _array_element _outactors
    (bind _asplayer_start (Utilities|Casting|CastToPlayerStart _array_element))
    (if (Actor|ActorHasTag _asplayer_start "Player1")
      (Variables|Default|SetPlayer%201%20Start _asplayer_start)
      (elif (Actor|ActorHasTag _asplayer_start "Player2")
        (Variables|Default|SetPlayer%202%20Start _asplayer_start))))
  ;;[1 1 1] Grab the player bodies
  (bind _outactors_2 (Actor|GetAllActorsOfClass "/Game/Assets/VR/Oculus_Character_Actor.Oculus_Character_Actor_C"))
  (for _array_element_2 _outactors_2
    (bind _asoculus_character_actor (Utilities|Casting|CastToOculus_Character_Actor _array_element_2))
    (if (Actor|ActorHasTag _asoculus_character_actor "PLayer1")
      (Variables|Default|SetPlayer%201%20Body _asoculus_character_actor)
      (elif (Actor|ActorHasTag _asoculus_character_actor "Player2")
        (Variables|Default|SetPlayer%202%20Body _asoculus_character_actor))))
  ;;[1 1 1] Grab the scoreboard
  (bind _outactors_3 (Actor|GetAllActorsOfClass "/Game/Blueprints/ScoreBoard/BP_Scoreboard.BP_Scoreboard_C"))
  (Variables|Default|SetScoreboard (Utilities|Array|Get(acopy) _outactors_3)))

(fn ConstructionScript)

(fn SelectBody
  (params (Player :type Oculus%20Player%20Controller%20Object%20Reference))
  (bind _player_1_body (Variables|Default|GetPlayer%201%20Body))
  (bind _player_2_body (Variables|Default|GetPlayer%202%20Body))
  (bind _player_2 (Variables|Default|GetPlayer%202))
  (bind _returnvalue (== Player _player_2))
  (bind _returnvalue_2 (select _returnvalue _player_2_body _player_1_body))
  (Variables|/Game/Assets/VR/Oculus_Character_Actor.Oculus_Character_Actor_C|SetIsTaken _returnvalue_2 true)
  (return _returnvalue_2))

(fn SpawnandPossessPlayer
  (params (PlayerController :type Player%20Controller%20Object%20Reference)))