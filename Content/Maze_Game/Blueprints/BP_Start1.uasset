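; BP_Start1 is a star pickup for the maze game that rewards the player when touched.
; Any overlap with its Sphere plays a pickup sound, then a cast limits the rest to BP_Player_Character_Pawn.
; The player gains a star and 500 score, and a pixel-bomb particle burst spawns at the pickup.
; After a brief delay, the emitter is deactivated and the actor destroys itself.
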(event OnComponentBeginOverlap(Sphere)
  (params (OverlappedComponent :type Primitive%20Component%20Object%20Reference) (OtherActor :type Actor%20Object%20Reference) (OtherComp :type Primitive%20Component%20Object%20Reference) (OtherBodyIndex :type Integer) (bFromSweep :type Boolean) (SweepResult :type Hit%20Result%20Structure%20%28by%20ref%29))
  (Audio|PlaySound2D "/Game/Maze_Game/Sound/Take/Key_Pickup02_Cue.Key_Pickup02_Cue" 1.0 1.0 0.0 0 0)
  (bind _asbp_player_character_pawn (Utilities|Casting|CastToBP_Player_Character_Pawn OtherActor))
  (Default|AddStar _asbp_player_character_pawn)
  (Variables|/Game/Blueprints/Game/BP_Player_Character_Pawn.BP_Player_Character_Pawn_C|SetScore _asbp_player_character_pawn (+ (Variables|/Game/Blueprints/Game/BP_Player_Character_Pawn.BP_Player_Character_Pawn_C|GetScore _asbp_player_character_pawn) 500))
  (bind _returnvalue (Effects|SpawnEmitteratLocation "/Game/Maze_Game/Particles/P_PixelBomb.P_PixelBomb" (Transformation|GetActorLocation) "0, 0, 0" "0.500000,0.500000,0.500000" false))
  (Utilities|FlowControl|Delay 0.1)
  (Components|Activation|Deactivate _returnvalue)
  (Actor|DestroyActor))

(event EventBeginPlay)

(event Collision|EventActorBeginOverlap
  (params (OtherActor :type Actor%20Object%20Reference)))

(event EventTick
  (params (DeltaSeconds :type Float%20%28single-precision%29)))

(fn ConstructionScript)