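; FallingFloor is a maze floor tile that gives way after the BP_UserBall rolls off it twice.
; Each end overlap on its Box calls TouchNumber and Fall through a FallingFloors reference.
; TouchNumber counts hits, swaps the floor material and sets Falling on the second hit.
; Fall then enables gravity on the mesh, which is destroyed after a short delay, with debug prints along the way.
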(event OnComponentEndOverlap(Box)
  (params (OtherActor :type Actor%20Object%20Reference) (OtherComp :type Primitive%20Component%20Object%20Reference) (OtherBodyIndex :type Integer))
  (bind _fallingfloors (Variables|Default|GetFallingFloors))
  (bind _asbp_user_ball (Utilities|Casting|CastToBP_UserBall OtherActor))
  (Variables|Default|SetUser_Ball _asbp_user_ball)
  (CallFunction|TouchNumber _fallingfloors)
  (CallFunction|Fall _fallingfloors)
  (if (Variables|Default|GetFalling)
    (Utilities|FlowControl|Delay 1.0)
    (Components|DestroyComponent (Variables|Default|GetFallingFloor))))

(event Custom|Fall
  (bind _fallingfloor (Variables|Default|GetFallingFloor))
  ;[1 1 1] Fall
  (if (Variables|Default|GetFalling)
    (Development|PrintString "fall")
    (Physics|SetEnableGravity _fallingfloor true)
    (else
      (Physics|SetEnableGravity _fallingfloor false))))

(event Custom|Touch%20Number
  ;[1 1 1] Touch Number
  (bind _output_get (Variables|Default|SetTotalHitFloor (+ (Variables|Default|GetTotalHitFloor) 1)))
  (Development|PrintString (Utilities|String|ToString(Integer) _output_get))
  (Rendering|Material|SetMaterial (Variables|Default|GetFallingFloor) 0 "/Game/Maze_Game/Materials/M_Tron_Inst_R.M_Tron_Inst_R")
  (if (== (Variables|Default|GetTotalHitFloor) 2)
    (Variables|Default|SetFalling true)))

(event EventBeginPlay)

(event EventActorBeginOverlap
  (params (OtherActor :type Actor%20Object%20Reference)))

(event EventTick
  (params (DeltaSeconds :type Float%20%28single-precision%29)))

(fn ConstructionScript)